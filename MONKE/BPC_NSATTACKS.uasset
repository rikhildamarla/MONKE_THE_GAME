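; Component on BP_MONKE that runs its two-hit Nanasaber melee combo from the IA_NSATTACK input, gated by CanAttack.
; Attack indexes the opening and follow-up slash montages, each played behind a DoOnce and short delay.
; Presses during an attack are buffered in SaveAttack; NSATTACKCOMBO, not called within this graph, consumes the buffer to chain onward or calls STOPCOMBO to reset.
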(event Custom|NS%20ATTACK
  (if (Variables|Default|GetisAttacking)
    (Variables|Default|SetSaveAttack true)
    (else
      (Variables|Default|SetisAttacking true)
      (switch int (Variables|Default|Getattack)
        (:0
          (CallFunction|NSATTACK1))
        (:1
          (CallFunction|NSATTACK2))))))

(event Custom|NS%20ATTACK%20COMBO
  (if (Variables|Default|GetSaveAttack)
    (Variables|Default|SetSaveAttack false)
    (switch int (Variables|Default|Getattack)
      (:0
        (CallFunction|NSATTACK1))
      (:1
        (CallFunction|NSATTACK2)))
    (else
      (CallFunction|STOPCOMBO))))

(event Custom|STOP%20COMBO
  (Variables|Default|SetisAttacking false)
  (Variables|Default|Setattack 0))

(event Custom|NS%20ATTACK%201
  ;[1 1 1] NANASABER ATTACK 1
  (Utilities|FlowControl|DoOnce false :!label _label
    (:Completed
      (Utilities|FlowControl|Delay 0.1)
      (Animation|Montage|PlayMontage (Variables|Default|GetCharacterMesh) "/Game/MONKE/MONKE_ANIMS/WITH_NANA_SABER/NS_SLASH_INIT1_Montage.NS_SLASH_INIT1_Montage"
        (:then
          (Variables|Default|Setattack 1)
          (goto _label Reset))))))

(event Custom|NS%20ATTACK%202
  ;[1 1 1] NANASABER ATTACK 2
  (Utilities|FlowControl|DoOnce false :!label _label
    (:Completed
      (Utilities|FlowControl|Delay 0.1)
      (Animation|Montage|PlayMontage (Variables|Default|GetCharacterMesh) "/Game/MONKE/MONKE_ANIMS/WITH_NANA_SABER/NS_SLASH_FOLLOW_UP_Montage.NS_SLASH_FOLLOW_UP_Montage"
        (:then
          (Variables|Default|Setattack 2)
          (goto _label Reset))))))

(event Input|EnhancedActionEvents|EnhancedInputActionIA_NSATTACK
  (params (ActionValue :type Boolean) (ElapsedSeconds :type Float%20%28double-precision%29) (TriggeredSeconds :type Float%20%28double-precision%29) (InputAction :type Input%20Action%20Object%20Reference :default "/Game/ThirdPerson/Input/Actions/IA_NSATTACK.IA_NSATTACK"))
  (:Started
    (if (Variables|Default|GetcanAttack)
      (CallFunction|NSATTACK))))

(event EventBeginPlay
  (bind _asbp_monke (Utilities|Casting|CastToBP_MONKE (Components|GetOwner)))
  (Variables|Default|SetCharacterMesh (Variables|/Script/Engine.Character|GetMesh _asbp_monke)))
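; BP_NANA_SABER is a saber weapon with a glowing blade that extends and retracts with sound.
; Activate and Retract events play their cue, then loop on a 0.1 second Delay, interpolating the glow mesh's Z scale with VInterpTo.
; IsActivated flips only once the scale exactly matches its target.
; Tick keeps the idle hum playing while IsActivated is true and stops it otherwise.
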(event Custom|NANASABER_RETRACT
  (bind _saber_glowy (Variables|Default|GetSABER_GLOWY))
  (bind _relativescale3d (Variables|/Script/Engine.SceneComponent|GetRelativeScale3D _saber_glowy))
  (Audio|Components|Audio|Play (Variables|Default|GetNANASABER_CLOSE_G711_org__Cue) 0.0)
  (if (Utilities|Operators|EqualEqual _relativescale3d "1.000000,1.000000,0.000000" 0.0) :!label _label
    (Variables|Default|SetisActivated false)
    (else
      (Transformation|SetRelativeScale3D _saber_glowy (Math|Interpolation|VInterpTo _relativescale3d "1.000000,1.000000,0.000000" (Utilities|Time|GetWorldDeltaSeconds) 7.0))
      (Utilities|FlowControl|Delay 0.1)
      (goto _label))))

(event Custom|NANASABER_ACTIVATE
  (bind _saber_glowy (Variables|Default|GetSABER_GLOWY))
  (bind _relativescale3d (Variables|/Script/Engine.SceneComponent|GetRelativeScale3D _saber_glowy))
  (Audio|Components|Audio|Play (Variables|Default|GetNANASABER_ACTUATE_G711_org__Cue) 0.0)
  (if (Utilities|Operators|EqualEqual _relativescale3d "1.000000,1.000000,1.500000" 0.0) :!label _label
    (Variables|Default|SetisActivated true)
    (else
      (Transformation|SetRelativeScale3D _saber_glowy (Math|Interpolation|VInterpTo _relativescale3d "1.000000,1.000000,1.500000" (Utilities|Time|GetWorldDeltaSeconds) 7.0))
      (Utilities|FlowControl|Delay 0.1)
      (goto _label))))

(event EventTick
  (params (DeltaSeconds :type Float%20%28single-precision%29))
  (if (Variables|Default|GetisActivated)
    (if (not (Audio|Components|Audio|IsPlaying (Variables|Default|GetNANASABER_IDLE_HUM_G711_org__Cue)))
      (Audio|Components|Audio|Play (Variables|Default|GetNANASABER_IDLE_HUM_G711_org__Cue) 0.0))
    (else
      (Audio|Components|Audio|Stop (Variables|Default|GetNANASABER_IDLE_HUM_G711_org__Cue)))))

(fn ConstructionScript)